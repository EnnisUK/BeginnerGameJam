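; Actor component that marks and unmarks its owner, toggling an outline highlight through custom depth and stencil.
; MarkObject enables custom depth on the owner's static or skeletal mesh component, chosen by MeshType, and writes the given stencil value.
; UnmarkObejct takes no inputs, switches on MeshType, disables custom depth and resets the stencil.
; Only the component returned by GetComponentByClass is affected; an invalid one prints an error.
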(event Custom|MarkObject
  (params (MeshType :type E_MeshType%20Enum :default "NewEnumerator0") (Stencil%20Value :type Integer))
  (bind _returnvalue (Components|GetOwner))
  (bind _returnvalue_2 (Actor|GetComponentbyClass _returnvalue "/Script/Engine.SkeletalMeshComponent"))
  (bind _returnvalue_3 (Actor|GetComponentbyClass _returnvalue "/Script/Engine.StaticMeshComponent"))
  (switch Utilities|FlowControl|Switch|SwitchonE_MeshType MeshType
    (:NewEnumerator0
      ;[0 0 0] Turn On Outline for Static Mesh
      (Utilities|IsValid _returnvalue_3
        (:Is%20Valid
          (Rendering|SetRenderCustomDepth _returnvalue_3 true)
          (Rendering|SetCustomDepthStencilValue _returnvalue_3 Stencil%20Value))
        (:Is%20Not%20Valid
          (Development|PrintString "ERROR: Static Mesh Is Invalid!" true true "(R=1.000000,G=0.000000,B=0.000000,A=1.000000)"))))
    (:NewEnumerator1
      ;[0 0 0] Turn On Outline for Skeletal Mesh
      (Utilities|IsValid _returnvalue_2
        (:Is%20Valid
          (Rendering|SetRenderCustomDepth _returnvalue_2 true)
          (Rendering|SetCustomDepthStencilValue _returnvalue_2 Stencil%20Value))
        (:Is%20Not%20Valid
          (Development|PrintString "ERROR: Skeletal Mesh Is Invalid!" true true "(R=1.000000,G=0.000000,B=0.000000,A=1.000000)"))))))

(event Custom|UnmarkObejct
  (bind _returnvalue (Components|GetOwner))
  (bind _returnvalue_2 (Actor|GetComponentbyClass _returnvalue "/Script/Engine.StaticMeshComponent"))
  (bind _returnvalue_3 (Actor|GetComponentbyClass _returnvalue "/Script/Engine.SkeletalMeshComponent"))
  (switch Utilities|FlowControl|Switch|SwitchonE_MeshType (stale Custom|MarkObject MeshType)
    (:NewEnumerator0
      ;[0 0 0] Turn Off Outline for Static Mesh
      (Utilities|IsValid _returnvalue_2
        (:Is%20Valid
          (Rendering|SetRenderCustomDepth _returnvalue_2 false)
          (Rendering|SetCustomDepthStencilValue _returnvalue_2 0))
        (:Is%20Not%20Valid
          (Development|PrintString "ERROR: Static Mesh Is Invalid!" true true "(R=1.000000,G=0.000000,B=0.000000,A=1.000000)"))))
    (:NewEnumerator1
      ;[0 0 0] Turn Off Outline for Skeletal Mesh
      (Utilities|IsValid _returnvalue_3
        (:Is%20Valid
          (Rendering|SetRenderCustomDepth _returnvalue_3 false)
          (Rendering|SetCustomDepthStencilValue _returnvalue_3 0))
        (:Is%20Not%20Valid
          (Development|PrintString "ERROR: Skeletal Mesh Is Invalid!" true true "(R=1.000000,G=0.000000,B=0.000000,A=1.000000)"))))))