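; Elevator Blueprint that moves a lift between Start and End points when a BP_SmallRobot overlaps its trigger box.
; The MoveElevator timeline lerps the lift's relative location; on arrival the railing animates, then GoUp clears after a short delay.
; With GoUp false, an overlap plays the railing-up animation, waits, then reverses the timeline.
; Nothing in the graph sets GoUp back to true.
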(event OnComponentBeginOverlap(Box)
  (params (OverlappedComponent :type Primitive%20Component%20Object%20Reference) (OtherActor :type Actor%20Object%20Reference) (OtherComp :type Primitive%20Component%20Object%20Reference) (OtherBodyIndex :type Integer) (bFromSweep :type Boolean) (SweepResult :type Hit%20Result%20Structure%20%28by%20ref%29))
  (Utilities|Casting|CastToBP_SmallRobot OtherActor)
  (if (Variables|Default|GetGoUp?)
    (bind _move (Timeline|MoveElevator Play)
      (:Update
        (Transformation|SetRelativeLocation (Variables|Default|GetLift) (Math|Vector|Lerp(Vector) (Variables|Default|GetStart) (Variables|Default|GetEnd) _move) false false))
      (:Finished
        (if (Variables|Default|GetGoUp?)
          (|PlayAnimation_2 1.0 "/Game/BeginnerGameJamFolder/Environment/Mechanics/Elevator/RailingAnimation.RailingAnimation")
          (Utilities|FlowControl|Delay 1.0)
          (Variables|Default|SetGoUp? false))))
    (else
      (Components|Animation|PlayAnimation (Variables|Default|GetRailing) "/Game/BeginnerGameJamFolder/Environment/Mechanics/Elevator/RailingGoingUp.RailingGoingUp" false)
      (Utilities|FlowControl|Delay 1.0)
      (Timeline|MoveElevator Reverse))))

(event EventBeginPlay)

(event Collision|EventActorBeginOverlap
  (params (OtherActor :type Actor%20Object%20Reference)))

(event EventTick
  (params (DeltaSeconds :type Float%20%28single-precision%29)))

(fn ConstructionScript)