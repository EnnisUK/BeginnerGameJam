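; Pressure pad actor that opens a linked door while an object tagged Pickup overlaps it.
; Overlap begin and end notify the DoorToOpen reference through PadActivated and PadDeactivated.
; The MovePad timeline plays and reverses to lerp the pad mesh's relative height, sinking it when pressed and raising it when released.
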(event EventBeginPlay)

(event Collision|EventActorBeginOverlap
  (params (OtherActor :type Actor%20Object%20Reference))
  (if (Actor|ActorHasTag OtherActor "Pickup")
    (Default|PadActivated (Variables|Default|GetDoorToOpen))
    (bind _move (Timeline|MovePad Play)
      (:Update
        (Transformation|SetRelativeLocation (Variables|Default|GetPad1) (Math|Vector|Lerp(Vector) "0.000000,0.000000,9.000000" "0.000000,0.000000,3.000000" _move) false false)))))

(event EventTick
  (params (DeltaSeconds :type Float%20%28single-precision%29)))

(event Collision|EventActorEndOverlap
  (params (OtherActor :type Actor%20Object%20Reference))
  (if (Actor|ActorHasTag OtherActor "Pickup")
    (Default|PadDeactivated (Variables|Default|GetDoorToOpen))
    (bind _move (Timeline|MovePad Reverse)
      (:Update
        (Transformation|SetRelativeLocation (Variables|Default|GetPad1) (Math|Vector|Lerp(Vector) "0.000000,0.000000,9.000000" "0.000000,0.000000,3.000000" _move) false false)))))

(fn ConstructionScript)