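; Laser hazard actor that teleports the drone to a set location when it enters the beam's trigger box.
; A looping timer started on BeginPlay repeatedly spawns a Niagara beam at the actor's position, ending at EndVector.
; Each spawn also resizes the Box extents from EndVector plus padding.
; Box overlap casts to BP_Drone and moves it to NewLocation without sweeping.
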(event OnComponentBeginOverlap(Box)
  (params (OverlappedComponent :type Primitive%20Component%20Object%20Reference) (OtherActor :type Actor%20Object%20Reference) (OtherComp :type Primitive%20Component%20Object%20Reference) (OtherBodyIndex :type Integer) (bFromSweep :type Boolean) (SweepResult :type Hit%20Result%20Structure%20%28by%20ref%29))
  (bind _asbp_drone (Utilities|Casting|CastToBP_Drone OtherActor))
  (Transformation|SetActorLocation _asbp_drone (Variables|Default|GetNew%20Location) false false))

(event Custom|SpawnLaser
  (bind _endvector (Variables|Default|GetEndVector))
  (bind _returnvalue (Niagara|SpawnSystematLocation "/Game/BeginnerGameJamFolder/LaserLong.LaserLong" (Transformation|GetActorLocation) "0, 0, 0" "1.000000,1.000000,1.000000" false))
  (Variables|Default|SetLaserLong _returnvalue)
  (Effects|Components|ParticleSystem|SetVectorParameter (Variables|Default|GetLaserLong) "BeamEnd" (Variables|Default|GetEndVector))
  (Components|Box|SetBoxExtent (Variables|Default|GetBox) (Math|Vector|MakeVector (+ (.x _endvector) 2e+01) (+ (.y _endvector) 2e+01) (+ (.z _endvector) 2e+01)) true))

(event EventBeginPlay
  (Utilities|Time|SetTimerbyEvent (delegate Custom|SpawnLaser) 0.8 true))

(fn ConstructionScript)