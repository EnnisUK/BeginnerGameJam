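; BP_PadDoor is a sci-fi door that opens while enough pressure pads are active and closes when the count drops below the requirement.
; PadActivated and PadDeactivated events adjust the active pad count and compare it to PressurePadsNeeded.
; Two DoOnce gates that reset each other keep open and close from repeating, each playing its skeletal mesh animation and switching the box collision between Ignore and Block.
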(event Custom|PadDeactivated
  (bind _box (Variables|Default|GetBox))
  (Math|Integer|DecrementInt (Variables|Default|GetPressurePadsActive)
    (:%20%20
      (if (>= (Variables|Default|GetPressurePadsActive) (Variables|Default|GetPressurePadsNeeded))
        (Utilities|FlowControl|DoOnce false :!label _label
          (:Completed
            (Components|Animation|PlayAnimation (Variables|Default|GetSkeletalMesh) "/Game/BeginnerGameJamFolder/Environment/Mechanics/Door/PowerNodeDoor/Lewis_SciFIDoor_Door_Open.Lewis_SciFIDoor_Door_Open" false)
            (Collision|SetCollisionResponsetoAllChannels _box "ECR_Ignore")
            (goto _label_2 Reset)))
        (else
          (Utilities|FlowControl|DoOnce false :!label _label_2
            (:Completed
              (Components|Animation|PlayAnimation (Variables|Default|GetSkeletalMesh) "/Game/BeginnerGameJamFolder/Environment/Mechanics/Door/PowerNodeDoor/Lewis_SciFIDoor_Door_Close.Lewis_SciFIDoor_Door_Close" false)
              (Collision|SetCollisionResponsetoAllChannels _box "ECR_Block")
              (goto _label Reset))))))))

(event Custom|PadActivated
  (bind _box (Variables|Default|GetBox))
  (Math|Integer|IncrementInt (Variables|Default|GetPressurePadsActive)
    (:%20%20
      (if (>= (Variables|Default|GetPressurePadsActive) (Variables|Default|GetPressurePadsNeeded))
        (Utilities|FlowControl|DoOnce false :!label _label
          (:Completed
            (Components|Animation|PlayAnimation (Variables|Default|GetSkeletalMesh) "/Game/BeginnerGameJamFolder/Environment/Mechanics/Door/PowerNodeDoor/Lewis_SciFIDoor_Door_Open.Lewis_SciFIDoor_Door_Open" false)
            (Collision|SetCollisionResponsetoAllChannels _box "ECR_Ignore")
            (goto _label_2 Reset)))
        (else
          (Utilities|FlowControl|DoOnce false :!label _label_2
            (:Completed
              (Components|Animation|PlayAnimation (Variables|Default|GetSkeletalMesh) "/Game/BeginnerGameJamFolder/Environment/Mechanics/Door/PowerNodeDoor/Lewis_SciFIDoor_Door_Close.Lewis_SciFIDoor_Door_Close" false)
              (Collision|SetCollisionResponsetoAllChannels _box "ECR_Block")
              (goto _label Reset))))))))

(event EventBeginPlay)

(event Collision|EventActorBeginOverlap
  (params (OtherActor :type Actor%20Object%20Reference)))

(event EventTick
  (params (DeltaSeconds :type Float%20%28single-precision%29)))

(fn ConstructionScript)