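; BP_PowerNodeDoor is an interactable sci-fi door that opens once the required number of power nodes has been hit.
; On BeginPlay it caches GameJam_GM, which holds the PowerNodeHit count.
; Interact prints a debug string and requires that count to exactly equal PowerNeeded.
; A DoOnce then plays the door's open animation and resets the shared count to zero.
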(event EventBeginPlay
  (bind _asgame_jam_gm (Utilities|Casting|CastToGameJam_GM (Game|GetGameMode)))
  (Variables|Default|SetAs%20Game%20Jam%20GM _asgame_jam_gm))

(event Collision|EventActorBeginOverlap
  (params (OtherActor :type Actor%20Object%20Reference)))

(event EventTick
  (params (DeltaSeconds :type Float%20%28single-precision%29)))

(event EventInteract
  (Development|PrintString "Hello")
  (if (== (Variables|/Game/BeginnerGameJamFolder/Systems/GameJam_GM.GameJam_GM_C|GetPowerNodeHit (Variables|Default|GetAs%20Game%20Jam%20GM)) (Variables|Default|GetPowerNeeded))
    (Utilities|FlowControl|DoOnce false
      (:Completed
        (Components|Animation|PlayAnimation (Variables|Default|GetDoorMesh) "/Game/BeginnerGameJamFolder/Environment/Mechanics/Door/Lewis_SciFIDoor_Door_Open.Lewis_SciFIDoor_Door_Open" false)
        (Variables|/Game/BeginnerGameJamFolder/Systems/GameJam_GM.GameJam_GM_C|SetPowerNodeHit (Variables|Default|GetAs%20Game%20Jam%20GM) 0)))))

(fn ConstructionScript)