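; SetNewText_BP is a trigger volume that gives the cat (Cat_BP) new dialogue when the player enters it.
; It fires once, after the game mode's TimesTalked count reaches TimesTalkedNeeded.
; It can first move the cat to one of two preset locations, chosen by teleport flags.
; It then pushes InputText to the cat's TalkToCatHUD, resets its talked state and calls ResetMeow.
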(event OnComponentBeginOverlap(Box)
  (params (OverlappedComponent :type Primitive%20Component%20Object%20Reference) (OtherActor :type Actor%20Object%20Reference) (OtherComp :type Primitive%20Component%20Object%20Reference) (OtherBodyIndex :type Integer) (bFromSweep :type Boolean) (SweepResult :type Hit%20Result%20Structure%20%28by%20ref%29))
  (Utilities|Casting|CastToBP_PlayerCharacter OtherActor)
  (if (>= (Variables|/Game/BeginnerGameJamFolder/Systems/GameJam_GM.GameJam_GM_C|GetTimesTalked (Variables|Default|GetAs%20Game%20Jam%20GM)) (Variables|Default|GetTimesTalkedNeeded))
    (Utilities|FlowControl|DoOnce false
      (:Completed
        (if (Variables|Default|GetShouldCatTeleport)
          (if (Variables|Default|GetFirstTeleport?)
            (Variables|Default|SetTPLocation (Variables|Default|GetFirstTPLocation))
            (bind _returnvalue (Transformation|SetActorLocation (Variables|Default|GetAs%20Cat%20BP) (Variables|Default|GetTPLocation) false false :!label _label))
            (if _returnvalue
              (Variables|Default|SetIndexTeleport (+ (Variables|Default|GetIndexTeleport) 1))
              (bind _returnvalue_2 (Actor|GetActorOfClass "/Game/BeginnerGameJamFolder/Characters/Cat/Cat_BP.Cat_BP_C" :!label _label_2))
              (bind _output_get (Variables|Default|SetAs%20Cat%20BP _returnvalue_2))
              (Variables|/Game/BeginnerGameJamFolder/HUD/Cat/TalkToCat.TalkToCat_C|SetInputText (Variables|/Game/BeginnerGameJamFolder/Characters/Cat/Cat_BP.Cat_BP_C|GetTalkToCatHUD _output_get) (Variables|Default|GetInput%20Text))
              (Variables|/Game/BeginnerGameJamFolder/HUD/Cat/TalkToCat.TalkToCat_C|SetCatHasSmthToSay (Variables|/Game/BeginnerGameJamFolder/Characters/Cat/Cat_BP.Cat_BP_C|GetTalkToCatHUD _output_get) true)
              (Variables|/Game/BeginnerGameJamFolder/HUD/Cat/TalkToCat.TalkToCat_C|SetAlreadyTalked? (Variables|/Game/BeginnerGameJamFolder/Characters/Cat/Cat_BP.Cat_BP_C|GetTalkToCatHUD _output_get) false)
              (Default|ResetMeow (Variables|/Game/BeginnerGameJamFolder/Characters/Cat/Cat_BP.Cat_BP_C|GetTalkToCatHUD _output_get)))
            (elif (Variables|Default|GetSecondTeleport)
              (Variables|Default|SetTPLocation (Variables|Default|GetSecondTpLocation))
              (goto _label)))
          (else
            (goto _label_2)))))))

(event EventBeginPlay
  (bind _asgame_jam_gm (Utilities|Casting|CastToGameJam_GM (Game|GetGameMode)))
  (Variables|Default|SetAs%20Game%20Jam%20GM _asgame_jam_gm)
  (bind _returnvalue (Actor|GetActorOfClass "/Game/BeginnerGameJamFolder/Characters/Cat/Cat_BP.Cat_BP_C"))
  (Variables|Default|SetAs%20Cat%20BP _returnvalue))

(event Collision|EventActorBeginOverlap
  (params (OtherActor :type Actor%20Object%20Reference)))

(fn ConstructionScript)