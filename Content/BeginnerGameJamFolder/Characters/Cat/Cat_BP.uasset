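; Cat_BP is a cat character that always faces the player and meows when interacted with.
; A fast looping timer snaps its rotation toward the player character using a look-at rotation.
; A second looping timer, with an interval randomized once at BeginPlay, plays a happy jump animation and then returns to walking.
; Interact plays a random meow from a sound array as 2D audio.
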(event Custom|Look%20At%20Player
  (bind _returnvalue (Game|GetPlayerCharacter 0))
  (Utilities|IsValid _returnvalue
    (:Is%20Valid
      (Transformation|SetActorRotation (Math|Rotator|FindLookatRotation (Transformation|GetActorLocation) (Transformation|GetActorLocation _returnvalue))))))

(event Custom|HappyJump
  (bind _mesh (Variables|Character|GetMesh))
  (Components|Animation|PlayAnimation _mesh "/Game/BeginnerGameJamFolder/Characters/Cat/Animations/HappyJump.HappyJump" false)
  (Utilities|FlowControl|Delay 0.7)
  (Components|Animation|PlayAnimation _mesh "/Game/BeginnerGameJamFolder/Characters/Cat/Animations/Walk.Walk" true))

(event EventBeginPlay
  (Utilities|Time|SetTimerbyEvent (delegate Custom|Look%20At%20Player) 0.01 true)
  (Utilities|Time|SetTimerbyEvent (delegate Custom|HappyJump) (Math|Random|RandomFloatinRange 5.0 15.0) true))

(event EventInteract
  (bind _returnvalue (Audio|CreateSound2D (Utilities|Array|Get(acopy) (Variables|Default|GetCatMeowArray) (Math|Random|RandomIntegerinRange 0 4)) 0.4 1.0 0.0 0))
  (Audio|Components|Audio|Play _returnvalue 0.0))

(fn ConstructionScript)