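; BP_PlayerCharacter is the player character, with a double jump, pause menu, cat dialogue and a swap into the last controlled robot stored in the GameMode.
; A looping timer runs a camera line trace that marks and unmarks actors implementing both the Mark and Interact interfaces.
; TalkBox overlaps show or remove a cat's chat widget, which the talk input advances or resets.
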(event OnComponentEndOverlap(TalkBox)
  (params (OverlappedComponent :type Primitive%20Component%20Object%20Reference) (OtherActor :type Actor%20Object%20Reference) (OtherComp :type Primitive%20Component%20Object%20Reference) (OtherBodyIndex :type Integer))
  (bind _as_cat_bp (Variables|Default|GetAs%20Cat%20BP))
  (bind _talktocathud (Variables|/Game/BeginnerGameJamFolder/Characters/Cat/Cat_BP.Cat_BP_C|GetTalkToCatHUD _as_cat_bp))
  (bind _ascat_bp (Utilities|Casting|CastToCat_BP OtherActor))
  (Variables|Default|SetTalkToCat? false)
  (Utilities|IsValid (Variables|/Game/BeginnerGameJamFolder/Characters/Cat/Cat_BP.Cat_BP_C|GetTalkToCatHUD _ascat_bp)
    (:Is%20Valid
      (Widget|RemovefromParent (Variables|/Game/BeginnerGameJamFolder/Characters/Cat/Cat_BP.Cat_BP_C|GetTalkToCatHUD _ascat_bp))
      (Widget|SetVisibility (Variables|/Game/BeginnerGameJamFolder/HUD/Cat/TalkToCat.TalkToCat_C|GetFToTalk (Variables|/Game/BeginnerGameJamFolder/Characters/Cat/Cat_BP.Cat_BP_C|GetTalkToCatHUD _ascat_bp)) "Hidden")
      (if (not (Variables|/Game/BeginnerGameJamFolder/HUD/Cat/TalkToCat.TalkToCat_C|GetCatHasSmthToSay _talktocathud))
        (Default|Reset _talktocathud)))))

(event OnComponentBeginOverlap(TalkBox)
  (params (OverlappedComponent :type Primitive%20Component%20Object%20Reference) (OtherActor :type Actor%20Object%20Reference) (OtherComp :type Primitive%20Component%20Object%20Reference) (OtherBodyIndex :type Integer) (bFromSweep :type Boolean) (SweepResult :type Hit%20Result%20Structure%20%28by%20ref%29))
  (bind _ascat_bp (Utilities|Casting|CastToCat_BP OtherActor))
  (Variables|Default|SetAs%20Cat%20BP _ascat_bp)
  (if (Variables|/Game/BeginnerGameJamFolder/HUD/Cat/TalkToCat.TalkToCat_C|GetCatHasSmthToSay (Variables|/Game/BeginnerGameJamFolder/Characters/Cat/Cat_BP.Cat_BP_C|GetTalkToCatHUD _ascat_bp))
    (Variables|Default|SetTalkToCat? true)
    (UserInterface|Viewport|AddtoViewport (Variables|/Game/BeginnerGameJamFolder/Characters/Cat/Cat_BP.Cat_BP_C|GetTalkToCatHUD _ascat_bp) 0)
    (Widget|SetVisibility (Variables|/Game/BeginnerGameJamFolder/HUD/Cat/TalkToCat.TalkToCat_C|GetFToTalk (Variables|/Game/BeginnerGameJamFolder/Characters/Cat/Cat_BP.Cat_BP_C|GetTalkToCatHUD _ascat_bp)) "Visible")))

(event Custom|MarkTrace
  (CallFunction|MarkFunction))

(event Input|EnhancedActionEvents|EnhancedInputActionIA_Talk
  (params (ActionValue :type Boolean) (ElapsedSeconds :type Float%20%28double-precision%29) (TriggeredSeconds :type Float%20%28double-precision%29) (InputAction :type Input%20Action%20Object%20Reference :default "/Game/BeginnerGameJamFolder/Input/Player/Actions/IA_Talk.IA_Talk"))
  (bind _as_cat_bp (Variables|Default|GetAs%20Cat%20BP))
  (bind _talktocathud (Variables|/Game/BeginnerGameJamFolder/Characters/Cat/Cat_BP.Cat_BP_C|GetTalkToCatHUD _as_cat_bp))
  (:Triggered
    (if (Variables|Default|GetTalkToCat?)
      (Utilities|IsValid _as_cat_bp
        (:Is%20Valid
          (Widget|SetVisibility (Variables|/Game/BeginnerGameJamFolder/HUD/Cat/TalkToCat.TalkToCat_C|GetTextChatBorder _talktocathud) "Visible")
          (Widget|SetVisibility (Variables|/Game/BeginnerGameJamFolder/HUD/Cat/TalkToCat.TalkToCat_C|GetFToTalk _talktocathud) "Hidden")
          (if (Variables|/Game/BeginnerGameJamFolder/HUD/Cat/TalkToCat.TalkToCat_C|GetNextText? _talktocathud)
            (Default|StartTalking _talktocathud)
            (elif (not (Variables|/Game/BeginnerGameJamFolder/HUD/Cat/TalkToCat.TalkToCat_C|GetCatHasSmthToSay _talktocathud))
              (Default|Reset _talktocathud))))))))

(event Input|EnhancedActionEvents|EnhancedInputActionIA_PossessPlayer
  (params (ActionValue :type Boolean) (ElapsedSeconds :type Float%20%28double-precision%29) (TriggeredSeconds :type Float%20%28double-precision%29) (InputAction :type Input%20Action%20Object%20Reference :default "/Game/BeginnerGameJamFolder/Input/Player/Actions/IA_PossessPlayer.IA_PossessPlayer"))
  (bind _returnvalue (Game|GetPlayerController 0))
  (bind _as_game_jam_gm (Variables|Default|GetAs%20Game%20Jam%20GM))
  (bind _lastcontrolledrobot (Variables|/Game/BeginnerGameJamFolder/Systems/GameJam_GM.GameJam_GM_C|GetLastControlledRobot _as_game_jam_gm))
  (:Triggered
    (if (Pawn|IsPlayerControlled)
      (Utilities|IsValid _lastcontrolledrobot
        (:Is%20Valid
          (Pawn|UnPossess _returnvalue)
          (Pawn|Possess _returnvalue _lastcontrolledrobot))))))

(event EventBeginPlay
  (bind _returnvalue (UserInterface|CreateWidget "/Game/BeginnerGameJamFolder/HUD/PauseMenu/PauseMenu.PauseMenu_C"))
  (Variables|Default|SetPauseMenuRef _returnvalue)
  (Utilities|Time|SetTimerbyEvent (delegate Custom|MarkTrace) 0.1 true)
  (bind _asgame_jam_gm (Utilities|Casting|CastToGameJam_GM (Game|GetGameMode)))
  (Variables|Default|SetAs%20Game%20Jam%20GM _asgame_jam_gm))

(event Collision|EventActorBeginOverlap
  (params (OtherActor :type Actor%20Object%20Reference)))

(event EventOnLanded
  (params (Hit :type Hit%20Result%20Structure%20%28by%20ref%29))
  (Utilities|FlowControl|DoN 2) ; enters at Reset
)

(event Input|ActionEvents|InputActionJump
  (params (Key :type Key%20Structure :default "None"))
  (:Pressed
    (Utilities|FlowControl|DoN 2
      (:Exit
        (Character|LaunchCharacter (Math|Vector|MakeVector 0.0 0.0 (Variables|/Script/Engine.CharacterMovementComponent|GetJumpZVelocity (Variables|Character|GetCharacterMovement))) false true)))))

(event Input|ActionEvents|InputActionPauseMenu
  (params (Key :type Key%20Structure :default "None"))
  (bind _returnvalue (Game|GetPlayerController 0))
  (bind _pausemenuref (Variables|Default|GetPauseMenuRef))
  (:Pressed
    (Utilities|IsValid _pausemenuref
      (:Is%20Valid
        (UserInterface|Viewport|AddtoViewport _pausemenuref 0)
        (Input|DisableInput _returnvalue)
        (Variables|/Script/Engine.PlayerController|SetbShowMouseCursor _returnvalue true)
        (Input|SetInputModeUIOnly _returnvalue 0 "DoNotLock" false)))))

(fn ConstructionScript)

(fn MarkFunction
  (bind _camera (Variables|Default|GetCamera))
  (bind _returnvalue (Transformation|GetWorldLocation _camera))
  (bind (_outhit _returnvalue_2) (Collision|LineTraceByChannel _returnvalue (+ _returnvalue (* (Math|Vector|GetForwardVector (Transformation|GetWorldRotation _camera)) (Variables|Default|GetTraceDistance))) "TraceTypeQuery1" false 0 "None"))
  (if _returnvalue_2
    (if (and (Utilities|DoesObjectImplementInterface (.HitActor (Collision|BreakHitResult _outhit)) "/Game/BeginnerGameJamFolder/Systems/Mark.Mark_C") (Utilities|DoesObjectImplementInterface (.HitActor (Collision|BreakHitResult _outhit)) "/Script/BeginnerGameJam.InteractInterface"))
      (Variables|Default|SetHit%20Actor (.HitActor (Collision|BreakHitResult _outhit)))
      (Utilities|FlowControl|DoOnce false :!label _label
        (:Completed
          (Class|Mark|Mark(Message) (Variables|Default|GetHit%20Actor))))
      (else
        (Class|Mark|UnMark(Message) (Variables|Default|GetHit%20Actor) :!label _label_2)
        (Variables|Default|SetHit%20Actor 0)
        (goto _label Reset)))
    (else
      (goto _label_2))))