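; Small robot character that the player can possess through Interact once the game mode's TimesTalked reaches three, returning control to the player character on input or destruction.
; While controlled, a looping timer runs a camera trace that highlights Pickup-tagged actors through the Mark interface.
; Grab attaches an overlapping pickup to a mesh socket or drops it via a ground trace, with special vent handling.
; It also handles single jumps and pausing.
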(event Custom|Trace
  (if (Pawn|IsPlayerControlled)
    (CallFunction|MarkFunction)))

(event Input|EnhancedActionEvents|EnhancedInputActionIA_PossessPlayer
  (params (ActionValue :type Boolean) (ElapsedSeconds :type Float%20%28double-precision%29) (TriggeredSeconds :type Float%20%28double-precision%29) (InputAction :type Input%20Action%20Object%20Reference :default "/Game/BeginnerGameJamFolder/Input/Player/Actions/IA_PossessPlayer.IA_PossessPlayer"))
  (bind _returnvalue (Game|GetPlayerController 0))
  (:Triggered
    (bind _returnvalue_2 (Actor|GetActorOfClass "/Game/BeginnerGameJamFolder/Characters/Player/BP_PlayerCharacter.BP_PlayerCharacter_C"))
    (Pawn|UnPossess _returnvalue)
    (Pawn|Possess _returnvalue _returnvalue_2)
    (Pawn|Components|CharacterMovement|SetMovementMode (Variables|Character|GetCharacterMovement) "MOVE_Walking" 0)))

(event Input|EnhancedActionEvents|EnhancedInputActionIA_SmallRobot_Grab
  (params (ActionValue :type Boolean) (ElapsedSeconds :type Float%20%28double-precision%29) (TriggeredSeconds :type Float%20%28double-precision%29) (InputAction :type Input%20Action%20Object%20Reference :default "/Game/BeginnerGameJamFolder/Input/SmallRobot/IA_SmallRobot_Grab.IA_SmallRobot_Grab"))
  (:Triggered
    (if (Variables|Default|GetIsGrabing)
      (|Drop)
      (else
        (|PickupBox)))))

(event Collision|EventActorBeginOverlap
  (params (OtherActor :type Actor%20Object%20Reference)))

(event EventInteract
  (if (>= (Variables|/Game/BeginnerGameJamFolder/Systems/GameJam_GM.GameJam_GM_C|GetTimesTalked (Variables|Default|GetAs%20Game%20Jam%20GM)) 3)
    (CallFunction|LerpCamera self)
    (Utilities|FlowControl|Delay 0.5)
    (Pawn|Possess (Game|GetPlayerController 0) self)
    (Pawn|Components|CharacterMovement|SetMovementMode (Variables|Character|GetCharacterMovement) "MOVE_Walking" 0)
    (Variables|/Game/BeginnerGameJamFolder/Systems/GameJam_GM.GameJam_GM_C|SetLastControlledRobot (Variables|Default|GetAs%20Game%20Jam%20GM) self)))

(event EventDestroyed
  (bind _returnvalue (Actor|GetActorOfClass "/Game/BeginnerGameJamFolder/Characters/Player/BP_PlayerCharacter.BP_PlayerCharacter_C"))
  (Pawn|Possess (Game|GetPlayerController 0) _returnvalue))

(event EventBeginPlay
  (bind _asbp_player_character (Utilities|Casting|CastToBP_PlayerCharacter (Game|GetPlayerCharacter 0)))
  (Variables|Default|SetAs%20BP%20Player%20Character _asbp_player_character)
  (Utilities|Time|SetTimerbyEvent (delegate Custom|Trace) 0.1 true)
  (bind _asgame_jam_gm (Utilities|Casting|CastToGameJam_GM (Game|GetGameMode)))
  (Variables|Default|SetAs%20Game%20Jam%20GM _asgame_jam_gm))

(event Input|ActionEvents|InputActionPauseMenu
  (params (Key :type Key%20Structure :default "None"))
  (bind _returnvalue (Game|GetPlayerController 0))
  (bind _as_bp_player_character (Variables|Default|GetAs%20BP%20Player%20Character))
  (bind _pausemenuref (Variables|/Game/BeginnerGameJamFolder/Characters/Player/BP_PlayerCharacter.BP_PlayerCharacter_C|GetPauseMenuRef _as_bp_player_character))
  (:Pressed
    (Utilities|IsValid _pausemenuref
      (:Is%20Valid
        (UserInterface|Viewport|AddtoViewport _pausemenuref 0)
        (Input|DisableInput _returnvalue)
        (Variables|/Script/Engine.PlayerController|SetbShowMouseCursor _returnvalue true)
        (Input|SetInputModeUIOnly _returnvalue 0 "DoNotLock" false)))))

(fn ConstructionScript)

(fn MarkFunction
  (bind _camera (Variables|Default|GetCamera))
  (bind _returnvalue (Transformation|GetWorldLocation _camera))
  (bind (_outhit _returnvalue_2) (Collision|LineTraceByChannel _returnvalue (+ _returnvalue (* (Math|Vector|GetForwardVector (Transformation|GetWorldRotation _camera)) (Variables|Default|GetTraceDistance))) "TraceTypeQuery1" false 0 "None"))
  (if _returnvalue_2
    (if (and (Utilities|DoesObjectImplementInterface (.HitActor (Collision|BreakHitResult _outhit)) "/Game/BeginnerGameJamFolder/Systems/Mark.Mark_C") (Actor|ActorHasTag (.HitActor (Collision|BreakHitResult _outhit)) "Pickup"))
      (Variables|Default|SetHit%20Actor (.HitActor (Collision|BreakHitResult _outhit)))
      (Utilities|FlowControl|DoOnce false :!label _label
        (:Completed
          (Class|Mark|Mark(Message) (Variables|Default|GetHit%20Actor))))
      (else
        (Class|Mark|UnMark(Message) (Variables|Default|GetHit%20Actor) :!label _label_2)
        (Variables|Default|SetHit%20Actor 0)
        (goto _label Reset)))
    (else
      (goto _label_2))))

(event EventMark
  (Default|MarkObject (Variables|Default|GetBP_MarkObjectsComponent) "NewEnumerator1"))

(event EventUnMark
  (Default|UnmarkObejct (Variables|Default|GetBP_MarkObjectsComponent)))

(event EventOnLanded
  (params (Hit :type Hit%20Result%20Structure%20%28by%20ref%29))
  (Utilities|FlowControl|DoN 1) ; enters at Reset
)

(event Input|ActionEvents|InputActionJump
  (params (Key :type Key%20Structure))
  (:Pressed
    (Utilities|FlowControl|DoN 1
      (:Exit
        (Character|LaunchCharacter (Math|Vector|MakeVector 0.0 0.0 (Variables|/Script/Engine.CharacterMovementComponent|GetJumpZVelocity (Variables|Character|GetCharacterMovement))) false true)))))