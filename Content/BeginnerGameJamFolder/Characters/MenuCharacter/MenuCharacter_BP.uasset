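; MenuCharacter is the main-menu character that builds the menu UI and launches the tutorial level when Start is clicked.
; On BeginPlay it requires JamGameInstance, creates the main menu and a hidden settings widget, then sets UI-only input with a visible cursor.
; A looping timer repeatedly binds the Start button's click, which removes the main menu and opens RealTutorialLevel through a DoOnce guard.
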(event Custom|OnClicked_Event
  (Widget|RemovefromParent (Variables|Default|GetMainMenu))
  (Utilities|FlowControl|DoOnce false
    (:Completed
      (Game|OpenLevel(byName) "RealTutorialLevel"))))

(event Custom|StartClicked
  (EventDispatchers|AssignOnClicked (Variables|/Game/BeginnerGameJamFolder/HUD/MainMenu/MainMenu_HUD.MainMenu_HUD_C|GetStart (Variables|Default|GetMainMenu)) (delegate Custom|OnClicked_Event)))

(event EventBeginPlay
  (bind _returnvalue (Game|GetPlayerController 0))
  (Utilities|Casting|CastToJamGameInstance (Game|GetGameInstance))
  (bind _returnvalue_2 (UserInterface|CreateWidget "/Game/BeginnerGameJamFolder/HUD/MainMenu/SettingsMenu_HUD_2.SettingsMenu_HUD_2_C"))
  (bind _output_get (Variables|Default|SetSettingsMenu2 _returnvalue_2))
  (Widget|SetVisibility _output_get "Hidden")
  (bind _returnvalue_3 (UserInterface|CreateWidget "/Game/BeginnerGameJamFolder/HUD/MainMenu/MainMenu_HUD.MainMenu_HUD_C"))
  (bind _output_get_2 (Variables|Default|SetMainMenu _returnvalue_3))
  (UserInterface|Viewport|AddtoViewport _output_get_2 0)
  (Utilities|Time|SetTimerbyEvent (delegate Custom|StartClicked) 0.1 true)
  (Input|SetInputModeUIOnly _returnvalue (Variables|Default|GetMainMenu) "DoNotLock" false)
  (Variables|/Script/Engine.PlayerController|SetbShowMouseCursor _returnvalue true))

(event Collision|EventActorBeginOverlap
  (params (OtherActor :type Actor%20Object%20Reference)))

(event EventTick
  (params (DeltaSeconds :type Float%20%28single-precision%29)))

(fn ConstructionScript)