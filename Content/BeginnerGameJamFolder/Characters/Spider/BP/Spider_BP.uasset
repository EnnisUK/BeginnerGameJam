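; Spider character that keeps facing the player and waves when the player comes close.
; A looping timer set on BeginPlay turns the actor's yaw toward the player character every 0.01 seconds.
; Entering WaveCollision plays a one-shot wave animation and returns to looping idle after a delay, gated by a DoOnce that resets when the player leaves.
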(event OnComponentBeginOverlap(WaveCollision)
  (params (OverlappedComponent :type Primitive%20Component%20Object%20Reference) (OtherActor :type Actor%20Object%20Reference) (OtherComp :type Primitive%20Component%20Object%20Reference) (OtherBodyIndex :type Integer) (bFromSweep :type Boolean) (SweepResult :type Hit%20Result%20Structure%20%28by%20ref%29))
  (Utilities|Casting|CastToBP_PlayerCharacter OtherActor)
  (Utilities|FlowControl|DoOnce false
    (:Completed
      (Components|Animation|PlayAnimation (Variables|Character|GetMesh) "/Game/BeginnerGameJamFolder/Characters/Spider/wave.wave" false)
      (Utilities|FlowControl|Delay 2.5)
      (Components|Animation|PlayAnimation (Variables|Character|GetMesh) "/Game/BeginnerGameJamFolder/Characters/Spider/Idle.Idle" true))))

(event OnComponentEndOverlap(WaveCollision)
  (params (OverlappedComponent :type Primitive%20Component%20Object%20Reference) (OtherActor :type Actor%20Object%20Reference) (OtherComp :type Primitive%20Component%20Object%20Reference) (OtherBodyIndex :type Integer))
  (Utilities|Casting|CastToBP_PlayerCharacter OtherActor)
  (Utilities|FlowControl|DoOnce false) ; enters at Reset
)

(event Custom|Look%20At%20Player
  (bind _returnvalue (Game|GetPlayerCharacter 0))
  (Utilities|IsValid _returnvalue
    (:Is%20Valid
      (Transformation|SetActorRotation (Math|Rotator|MakeRotator 0.0 0.0 (.yaw (Math|Rotator|FindLookatRotation (Transformation|GetActorLocation) (Transformation|GetActorLocation _returnvalue))))))))

(event EventBeginPlay
  (Utilities|Time|SetTimerbyEvent (delegate Custom|Look%20At%20Player) 0.01 true))

(event Collision|EventActorBeginOverlap
  (params (OtherActor :type Actor%20Object%20Reference)))

(event EventTick
  (params (DeltaSeconds :type Float%20%28single-precision%29)))

(fn ConstructionScript)